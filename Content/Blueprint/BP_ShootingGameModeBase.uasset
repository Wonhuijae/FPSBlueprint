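; Game mode for a shooting game that runs the opening title screen and tracks the current and best score.
; BeginPlay shows the title widget for a short delay, swaps it for the score widget, switches to game-only input and loads the best score.
; AddScore accumulates points and saves any new best through a BP_Savegame slot.
; Loading falls back to zero when no valid save exists.
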(event `self.ReceiveBeginPlay`
  (bind _returnvalue (`GameplayStatics.GetPlayerController` 0))
  (bind _returnvalue_2 (`|CreateWidget` "/Game/Blueprint/WBP_Title.WBP_Title_C"))
  (`UserWidget.AddToViewport` _returnvalue_2 0)
  (`KismetSystemLibrary.Delay` 2.0)
  (`WidgetLayoutLibrary.RemoveAllWidgets`)
  (bind _returnvalue_3 (`|CreateWidget` "/Game/Blueprint/WBP_Score.WBP_Score_C"))
  (`UserWidget.AddToViewport` _returnvalue_3 0)
  (set `PlayerController.bShowMouseCursor` false _returnvalue)
  (`WidgetBlueprintLibrary.SetInputMode_GameOnly` _returnvalue)
  (`self.LoadBestScore`))

(fn `AddScore`
  (params (Value :type Integer))
  ;[1 1 1] Score에 Value(정수)를 누적
  (bind _output_get (set `self.Score` (+ Value (`self.Score`))))
  ;[1 1 1] Score가 Best Score보다 크다면 Best Score의 값을 갱신
  (if (> _output_get (`self.BestScore`))
    (set `self.BestScore` (`self.Score`))
    (`self.SaveBestScore`)))

(fn `LoadBestScore`
  (bind _returnvalue (`GameplayStatics.DoesSaveGameExist` (`self.ScoreData`)))
  (if _returnvalue
    (bind _returnvalue_2 (`GameplayStatics.LoadGameFromSlot` (`self.ScoreData`)))
    (bind _asbp_savegame (cast `/Game/Blueprint/BP_Savegame` _returnvalue_2)
      (:`then`
        (set `self.BestScore` (`/Game/Blueprint/BP_Savegame.SaveBestScore` _asbp_savegame)))
      (:`CastFailed`
        (set `self.BestScore` 0 :!label _label)))
    (else
      (goto _label))))

(fn `SaveBestScore`
  (`|ExecutionSequence`
    (:`then_0`
      ;[1 1 1] 1. SaveGame 클래스를 생성
      (bind _returnvalue (`GameplayStatics.CreateSaveGameObject` "/Game/Blueprint/BP_Savegame.BP_Savegame_C"))
      (set `self.SaveGameInstance` _returnvalue))
    (:`then_1`
      ;[1 1 1] 2. 저장: SaveGame 객체를 만들고, 객체의 속성에 저장할 값을 대입한다.
      (set `/Game/Blueprint/BP_Savegame.SaveBestScore` (`self.BestScore`) (`self.SaveGameInstance`)))
    (:`then_2`
      ;[1 1 1] 3. 2를 슬롯(파일)에 저장
      (`GameplayStatics.SaveGameToSlot` (`self.SaveGameInstance`) (`self.ScoreData`)))))

(fn `UserConstructionScript`)