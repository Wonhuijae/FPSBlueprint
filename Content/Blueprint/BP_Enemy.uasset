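; Enemy that flies in a straight line and damages the player on contact.
; BeginPlay locks its direction: 30% chance toward the player's position, otherwise its forward vector.
; Tick moves it via the Translate helper and rotates it to face that direction.
; Overlapping BP_Player plays explosion effects, calls DoDamage and destroys the enemy; a true result also destroys the player, pauses the game and shows WBP_GameOver.
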(event `self.ReceiveBeginPlay`
  ;[1 1 1 1 15] 적이 태어날 때(BeginPlay) 30%확률로 플레이어를 향하고 아니면 아래를 향함, 살아 있는 동안 태어날 때 정해진 방향으로 이동
  (if (< (`KismetMathLibrary.RandomIntegerInRange` 0 9) 3)
    (set `self.Direction` (`KismetMathLibrary.Normal` (- (`self.K2_GetActorLocation` (`GameplayStatics.GetPlayerPawn` 0)) (`self.K2_GetActorLocation`))))
    (else
      (set `self.Direction` (`self.GetActorForwardVector`)))))

(event `self.ReceiveTick`
  (params (DeltaSeconds :type "Float (single-precision)"))
  ;[1 1 1 1 15] 적이 태어날 때(BeginPlay) 30%확률로 플레이어를 향하고 아니면 아래를 향함, 살아 있는 동안 태어날 때 정해진 방향으로 이동
  (`self.Translate` (`self.Direction`) (`self.Speed`))
  ;[1 1 1] Enemy 방향 바꾸기(플레이어를 바라보도록 돌려줌)
  (`self.K2_SetActorRotation` (`KismetMathLibrary.MakeRotFromXZ` (`self.Direction`) (`self.GetActorUpVector`))))

(event `self.ReceiveActorBeginOverlap`
  (params (OtherActor :type "Actor Object Reference"))
  (bind _returnvalue (`GameplayStatics.GetPlayerController` 0))
  (bind _asbp_player (cast `/Game/Blueprint/BP_Player` OtherActor))
  (`GameplayStatics.SpawnEmitterAtLocation` "/Game/StarterContent/Particles/P_Explosion.P_Explosion" (`self.K2_GetActorLocation` _asbp_player) (struct) (2.0 2.0 2.0))
  (`GameplayStatics.PlaySound2D` "/Game/VFX/destruction.destruction" 1.0 1.0 0.0 null null)
  (bind _isdie (`/Game/Blueprint/BP_Player.Do Damage` _asbp_player 10))
  (if _isdie
    (`self.K2_DestroyActor` _asbp_player)
    (`KismetSystemLibrary.Delay` 0.2)
    (`self.K2_DestroyActor`)
    (`GameplayStatics.SetGamePaused` true)
    (bind _returnvalue_2 (`|CreateWidget` "/Game/Blueprint/WBP_GameOver.WBP_GameOver_C"))
    (`UserWidget.AddToViewport` _returnvalue_2 0)
    (set `PlayerController.bShowMouseCursor` true _returnvalue)
    (`WidgetBlueprintLibrary.SetInputMode_UIOnlyEx` _returnvalue null)
    (else
      (`self.K2_DestroyActor`))))

(fn `Translate`
  (params (Direction :type "Vector Structure") (Speed :type "Float (double-precision)"))
  (`self.K2_SetActorLocation` (+ (`self.K2_GetActorLocation`) (* Speed (`KismetMathLibrary.Normal` Direction) (`GameplayStatics.GetWorldDeltaSeconds`)))))

(fn `UserConstructionScript`)