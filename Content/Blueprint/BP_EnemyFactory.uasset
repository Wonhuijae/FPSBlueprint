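; BP_EnemyFactory is a spawner actor that periodically creates BP_Enemy instances at its Arrow component's transform.
; BeginPlay starts a looping timer by function name that calls MakeEnemy every MakeTime seconds.
; MakeEnemy spawns only while the player pawn is valid, and otherwise clears the timer so production stops once the player is gone.
; An older Tick-based accumulator and an event-based timer remain in the graph, unconnected.
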(event `Event Make Enemy`
  (`self.MakeEnemy`))

(event `self.ReceiveBeginPlay`
  (bind _returnvalue (`KismetSystemLibrary.K2_SetTimer` null "MakeEnemy" (`self.MakeTime`) true))
  (set `self.TimerHandleMakeEnemy` _returnvalue))

(event `self.ReceiveTick`
  (params (DeltaSeconds :type "Float (single-precision)"))
  ;[1 1 1] 시간이 흐르다가 현재 시간이 생성되면 적을 Arrow 위치에 스폰,
  ; 그리고 시간을 0으로 초기화
)

(fn `MakeEnemy`
  ;[1 1 1] 플레이어가 죽었다면 더 이상 적을 만들지 않는다
  (`/Engine/EditorBlueprintResources/StandardMacros.IsValid` (`GameplayStatics.GetPlayerPawn` 0)
    (:`Is Valid`
      (`|SpawnActorFromClass` "/Game/Blueprint/BP_Enemy.BP_Enemy_C" (`SceneComponent.K2_GetComponentToWorld` (`self.Arrow`)) "AlwaysSpawn" "MultiplyWithRoot" null null))
    (:`Is Not Valid`
      (`KismetSystemLibrary.K2_ClearAndInvalidateTimerHandle` (`self.TimerHandleMakeEnemy`)))))

(fn `UserConstructionScript`)